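; Weapon Blueprint that a player picks up by interacting, switching between a dropped physics item and an attached, held item.
; UpdateState runs on BeginPlay and after pickup, using the attach parent to toggle mesh physics and the collision profiles of the mesh and interaction volume.
; GetLeftHandIK exposes the mesh's LeftHand_IK socket in world space for left-hand placement.
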(event `self.ReceiveBeginPlay`
  (`self.Update State`))

(event `/Game/Blueprints/Item/EInteractable.On Interacted`
  (params (Player :type "/Game/Blueprints/PlayerCharacter/PlayerCharacter Object Reference"))
  (`/Game/Blueprints/PlayerCharacter/PlayerCharacter.Pick Up Weapon` Player self)
  (`self.Update State`))

(fn `Get Left Hand IK`
  (returns (`Return Value` :type "Transform Structure"))
  (return (`SceneComponent.GetSocketTransform` (`self.Mesh`) "LeftHand_IK" "RTS_World")))

(fn `Update State`
  (bind _mesh (`self.Mesh`))
  (`/Engine/EditorBlueprintResources/StandardMacros.IsValid` (`self.GetAttachParentActor`)
    (:`Is Valid`
      (`PrimitiveComponent.SetSimulatePhysics` _mesh false)
      (`SceneComponent.ResetRelativeTransform` _mesh)
      (`PrimitiveComponent.SetCollisionProfileName` _mesh "NoCollision" true)
      (`PrimitiveComponent.SetCollisionProfileName` (`self.Interaction Collision`) "NoCollision" true))
    (:`Is Not Valid`
      (`PrimitiveComponent.SetSimulatePhysics` _mesh true)
      (`PrimitiveComponent.SetCollisionProfileName` _mesh "ItemOnGround" true)
      (`PrimitiveComponent.SetCollisionProfileName` (`self.Interaction Collision`) "OverlapAllDynamic" true))))

(fn `UserConstructionScript`
  (`parent.UserConstructionScript`))