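; Base weapon Blueprint that can be picked up through interaction and leaves Attack as an empty event.
; Interaction calls the player's server pickup, with remote clients also calling pickup locally first.
; A replicated state, applied on BeginPlay and OnRep, toggles mesh physics and collision between on-ground and picked-up.
; It exposes the mesh as the interaction widget's attach point and its LeftHand_IK socket for hand IK.
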(event `self.ReceiveBeginPlay`
  (`self.Update State`))

(event `/Game/Blueprints/Item/Interactable.On Interacted`
  (params (Player :type "/Game/Blueprints/PlayerCharacter/PlayerCharacter Object Reference"))
  (`/Engine/EditorBlueprintResources/ActorMacros.Switch Has Authority`
    (:`Authority`
      _)
    (:`Remote`
      (`/Game/Blueprints/PlayerCharacter/PlayerCharacter.Pick Up Weapon` Player self)))
  (`/Game/Blueprints/PlayerCharacter/PlayerCharacter.SERVER Pick Up Weapon` Player self))

(event `Attack`)

(fn `Get Interaction Widget Attach To`
  (returns (`Attach To Component` :type "SceneComponent Object Reference"))
  (return (`self.Mesh`)))

(fn `Get Left Hand IK`
  (returns (`Return Value` :type "Transform Structure"))
  (return (`SceneComponent.GetSocketTransform` (`self.Mesh`) "LeftHand_IK" "RTS_World")))

(fn `OnRep_New State`
  (`self.Update State`))

(fn `Set New State`
  (params (`New State` :type "/Game/Blueprints/Weapon/Enums/EWeaponState Enum" :default "NewEnumerator0"))
  (if (not (`|EnumEquality` `New State` (`self.New State`)))
    (set `self.New State` `New State`)))

(fn `Update State`
  (bind _mesh (`self.Mesh`))
  (bind _output_get (set `self.Current State` (`self.New State`)))
  (switch `/Game/Blueprints/Weapon/Enums/EWeaponState` _output_get
    (:`NewEnumerator0`
      (`PrimitiveComponent.SetSimulatePhysics` _mesh true)
      (`PrimitiveComponent.SetCollisionProfileName` _mesh "ItemOnGround" true)
      (`PrimitiveComponent.SetCollisionProfileName` (`self.Interaction Collision`) "OverlapAllDynamic" true)
      (`SceneComponent.ResetRelativeTransform` (`self.Mesh`)))
    (:`NewEnumerator1`
      (`PrimitiveComponent.SetSimulatePhysics` _mesh false)
      (`PrimitiveComponent.SetCollisionProfileName` _mesh "NoCollision" true)
      (`PrimitiveComponent.SetCollisionProfileName` (`self.Interaction Collision`) "NoCollision" true)
      (`SceneComponent.ResetRelativeTransform` (`self.Mesh`)))))

(fn `UserConstructionScript`
  (`parent.UserConstructionScript`))