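; FireWeapon is a gun Blueprint that attaches a separate magazine to its mesh and fires hitscan shots.
; Attack traces from the muzzle socket out to the maximum range with debug drawing, but the hit result is unused.
; A delay derived from rounds per minute gates the next shot, and full-auto weapons loop while the parent PlayerCharacter is attacking.
; Clip ammo is filled at BeginPlay but never consumed here.
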(event `self.ReceiveBeginPlay`
  (`parent.ReceiveBeginPlay`)
  (`SkinnedMeshComponent.HideBoneByName` (`self.Mesh`) "b_gun_mag" "PBO_None")
  (set `self.Ammo In Clip` (`self.Clip Size`)))

(event `self.Attack`
  (`self.Cast Bullet Ray` :!label _label)
  (set `self.Can Attack Now` false)
  (`KismetSystemLibrary.Delay` (/ 60.0 (`self.Attack Rate`)))
  (set `self.Can Attack Now` true)
  (if (`self.Is Full Auto`)
    (bind _asplayer_character (cast `/Game/Blueprints/PlayerCharacter/PlayerCharacter` (`self.GetAttachParentActor`)))
    (if (`/Game/Blueprints/PlayerCharacter/PlayerCharacter.Is Attacking` _asplayer_character)
      (goto _label))))

(fn `Cast Bullet Ray`
  (bind (_returnvalue_location _returnvalue_rotation) (`KismetMathLibrary.BreakTransform` (`SceneComponent.GetSocketTransform` (`self.Mesh`) "Muzzle" "RTS_World")))
  (`KismetSystemLibrary.LineTraceSingle` :`Start` _returnvalue_location :`End` (+ _returnvalue_location (* (`KismetMathLibrary.GetForwardVector` _returnvalue_rotation) (`self.Max Firing Range`))) :`TraceChannel` "TraceTypeQuery1" :`DrawDebugType` "ForDuration"))

(fn `UserConstructionScript`
  (`parent.UserConstructionScript`)
  (`SceneComponent.K2_AttachToComponent` (`self.Mag`) (`self.Mesh`) "Mag_Attach" "SnapToTarget" "SnapToTarget" "SnapToTarget" true))