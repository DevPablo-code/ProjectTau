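; Base item actor that shows an on-screen interaction prompt while a player looks at it.
; On look start it creates a widget with the item's interaction text and the key bound to the Interact action, hosted in a screen-space WidgetComponent added at runtime.
; The component attaches to the scene root via a getter function and is destroyed when the look ends.
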(event `/Game/Blueprints/Item/EInteractable.On Looked At Start`
  (params (Player :type "/Game/Blueprints/PlayerCharacter/PlayerCharacter Object Reference"))
  (bind (_asplayer_controller _bsuccess) (cast `PlayerController` (`Pawn.GetController` Player) :!pure true))
  (if _bsuccess
    (`/Engine/EditorBlueprintResources/StandardMacros.IsValid` (`self.Interaction Widget Component`)
      (:`Is Not Valid`
        (bind _returnvalue (`self.Create Interaction Widget` _asplayer_controller))
        (bind _returnvalue_2 (`AddComponent|NODE_AddWidgetComponent-0` :`bManualAttachment` true))
        (bind _output_get (set `self.Interaction Widget Component` _returnvalue_2))
        (`WidgetComponent.SetWidget` _output_get _returnvalue)
        (`WidgetComponent.SetWidgetSpace` _output_get "Screen")
        (`WidgetComponent.SetDrawAtDesiredSize` _output_get true)
        (`PrimitiveComponent.SetCollisionEnabled` _output_get "NoCollision")
        (`SceneComponent.K2_AttachToComponent` _output_get (`self.Get Interaction Widget Attach To`) "None" "SnapToTarget" "SnapToTarget" "SnapToTarget" true)))))

(event `/Game/Blueprints/Item/EInteractable.On Looked At End`
  (bind _interaction_widget_component (`self.Interaction Widget Component`)
    (:`then`
      (`ActorComponent.K2_DestroyComponent` _interaction_widget_component))
    (:`else`)))

(fn `Create Interaction Widget`
  (params (`Player Controller` :type "PlayerController Object Reference"))
  (returns (ReturnValue :type "/Game/Blueprints/Item/InteractionWidget Object Reference"))
  (bind (_output_actionname _output_bshift _output_bctrl _output_balt _output_bcmd _output_key) (break `InputActionKeyMapping` (`|GetArrayItem` (`InputSettings.GetActionMappingByName` (`InputSettings.GetInputSettings`) "Interact"))))
  (bind _returnvalue (`|CreateWidget` "/Game/Blueprints/Item/InteractionWidget.InteractionWidget_C" `Player Controller` (`KismetInputLibrary.Key_GetDisplayName` _output_key) (`self.Interaction Text`)))
  (return _returnvalue))

(fn `Get Interaction Widget Attach To`
  (returns (`Attach To Component` :type "SceneComponent Object Reference"))
  (return (`self.DefaultSceneRoot`)))

(fn `UserConstructionScript`)